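; Player state Blueprint that tracks a player's Health, Armor and Ammo.
; On BeginPlay it caches the game state cast to BP_CombatLogGameState.
; Add functions adjust each stat and call its update notification.
; DealDamage is meant to drain Armor before Health, but subtracts a literal zero, zeroes Armor before computing the overflow, and calls the Ammo update instead of the Armor one.
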(event `self.ReceiveBeginPlay`
  (bind _asbp_combat_log_game_state (cast `/Game/BP_CombatLogGameState` (`GameplayStatics.GetGameState`)))
  (set `self.GameState` _asbp_combat_log_game_state))

(event `self.ReceiveTick`
  (params (DeltaSeconds :type "Float (single-precision)")))

(fn `AddAmmo`
  (params (Amount :type Integer))
  (set `self.Ammo` (+ Amount (`self.Ammo`)))
  (`self.OnAmmoUpdate`))

(fn `AddArmor`
  (params (Amount :type Integer))
  (set `self.Armor` (+ Amount (`self.Armor`)))
  (`self.OnArmorUpdate`))

(fn `AddHealth`
  (params (Amount :type Integer))
  (set `self.Health` (+ Amount (`self.Health`)))
  (`self.OnHealthUpdate`))

(fn `DealDamage`
  (bind _returnvalue (- (`self.Armor`) 0))
  (if (< _returnvalue 0)
    (set `self.Armor` 0)
    (set `self.Health` (+ _returnvalue (`self.Health`)))
    (`self.OnHealthUpdate`)
    (else
      (set `self.Armor` _returnvalue)))
  (`self.OnAmmoUpdate`))

(fn `UserConstructionScript`)